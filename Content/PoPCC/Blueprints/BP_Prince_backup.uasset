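; Player character Blueprint for the Prince, handling Enhanced Input movement, camera look, crouch, roll and mantle.
; Crouch uses timelines to blend capsule height and camera arm length, with an upward sphere trace blocking uncrouch under obstacles.
; Mantle sweeps forward traces upward to find clearance, then traces down for the ledge.
; The hit sets a Motion Warping target for a 1M or 2M montage, chosen by distance, played in Flying mode.
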(event `self.ReceiveBeginPlay`
  ;[1 1 1] Main movement mapping input
  (`EnhancedInputSubsystemInterface.AddMappingContext` (pcsubsystem `EnhancedInputLocalPlayerSubsystem` (`GameplayStatics.GetPlayerController` 0)) "/Game/PoPCC/Input/IMC_PoPInput.IMC_PoPInput" 0 (struct)))

(event `EnhancedInput|/Game/PoPCC/Input/IA_Movement`
  (params (ActionValue :type "Vector2D Structure") (ElapsedSeconds :type "Float (double-precision)") (TriggeredSeconds :type "Float (double-precision)") (InputAction :type "InputAction Object Reference" :default "/Game/PoPCC/Input/IA_Movement.IA_Movement"))
  ;[1 1 1] X&Y Movement
  (:`Triggered`
    (`self.AddMovementInput` (`KismetMathLibrary.GetRightVector` (`self.GetControlRotation`)) ActionValue_X)
    (`self.AddMovementInput` (`KismetMathLibrary.GetForwardVector` (`self.GetControlRotation`)) ActionValue_Y)))

(event `EnhancedInput|/Game/PoPCC/Input/IA_Looking`
  (params (ActionValue :type "Vector2D Structure") (ElapsedSeconds :type "Float (double-precision)") (TriggeredSeconds :type "Float (double-precision)") (InputAction :type "InputAction Object Reference" :default "/Game/PoPCC/Input/IA_Looking.IA_Looking"))
  ;[1 1 1] Mouse Camera Movement
  (:`Triggered`
    (`self.AddControllerYawInput` ActionValue_X)
    (`self.AddControllerPitchInput` (* ActionValue_Y -1.0))))

(event `EnhancedInput|/Game/PoPCC/Input/IA_Crouching`
  (params (ActionValue :type Boolean) (ElapsedSeconds :type "Float (double-precision)") (TriggeredSeconds :type "Float (double-precision)") (InputAction :type "InputAction Object Reference" :default "/Game/PoPCC/Input/IA_Crouching.IA_Crouching"))
  (bind _charactermovement (`self.CharacterMovement`))
  ;[1 1 1] Crouched Movement & Camera
  (:`Started`
    (if (not (`self.IsCrouching`))
      (set `self.IsCrouching` true)
      (set `CharacterMovementComponent.MaxWalkSpeed` 350.0 _charactermovement)
      (`|ExecutionSequence`
        (:`then_0`
          (bind (_direction _arm_length) (`Timeline|Crouched Zoom Out` :!label _label)
            (:`Update`
              (set `SpringArmComponent.TargetArmLength` (`KismetMathLibrary.Lerp` 600.0 750.0 _arm_length) (`self.SpringArm`)))))
        (:`then_1`
          (bind (_direction_2 _capsule_height) (`Timeline|Crouched Capsule Height` :!label _label_2)
            (:`Update`
              (`CapsuleComponent.SetCapsuleHalfHeight` (`self.CapsuleComponent`) (`KismetMathLibrary.Lerp` 88.0 50.0 _capsule_height) true)
              (`SceneComponent.K2_SetRelativeLocation` (`self.Mesh`) (`KismetMathLibrary.MakeVector` 0.0 0.0 (`KismetMathLibrary.Lerp` -89.0 -49.0 _capsule_height)) false false)))))
      (else
        ;;[1 1 1] stop crouching if there is no obstacle
        (bind _foundobstacle (`self.Uncrouch Obstacle`))
        (if (not _foundobstacle)
          (set `self.IsCrouching` false)
          (set `CharacterMovementComponent.MaxWalkSpeed` 600.0 _charactermovement)
          (`|ExecutionSequence`
            (:`then_0`
              (goto _label :!via `Reverse`))
            (:`then_1`
              (goto _label_2 :!via `Reverse`))))))))

(event `EnhancedInput|/Game/PoPCC/Input/IA_Roll`
  (params (ActionValue :type Boolean) (ElapsedSeconds :type "Float (double-precision)") (TriggeredSeconds :type "Float (double-precision)") (InputAction :type "InputAction Object Reference" :default "/Game/PoPCC/Input/IA_Roll.IA_Roll"))
  ;[1 1 1] Roll Dodge
  (:`Started`
    (if (not (`self.IsRolling`))
      (`|PlayMontage` (`self.Mesh`) "/Game/PoPCC/Characters/Prince/Animations/Roll/Roll_Montage.Roll_Montage"
        (:`then`
          (set `self.IsRolling` true))
        (:`OnCompleted`
          (set `self.IsRolling` false))))))

(event `EnhancedInput|/Game/PoPCC/Input/IA_Mantle`
  (params (ActionValue :type Boolean) (ElapsedSeconds :type "Float (double-precision)") (TriggeredSeconds :type "Float (double-precision)") (InputAction :type "InputAction Object Reference" :default "/Game/PoPCC/Input/IA_Mantle.IA_Mantle"))
  (bind (_returnvalue_x _returnvalue_y) (`KismetMathLibrary.BreakVector` (`self.GetActorForwardVector`)))
  (bind _charactermovement (`self.CharacterMovement`))
  (bind _mesh (`self.Mesh`))
  ;[1 1 1] Mantle
  (:`Started`
    (if (and (not (`NavMovementComponent.IsFalling` (`self.CharacterMovement`))) (not (`self.IsMantling`)))
      ;;[1 1 1] Trace Forward
      (for _index (range (+ (`KismetMathLibrary.SelectInt` 7 4 (`self.IsCrouching`)) 1))
        (bind _returnvalue (+ (`self.K2_GetActorLocation`) (`KismetMathLibrary.MakeVector` 0.0 0.0 (* _index 30))))
        (bind (_outhit _returnvalue_2) (`KismetSystemLibrary.SphereTraceSingle` :`Start` _returnvalue :`End` (+ _returnvalue (* (`self.GetActorForwardVector`) 120.0)) :`Radius` 10.0 :`TraceChannel` "TraceTypeQuery1" :`DrawDebugType` "ForDuration"))
        (if (not _returnvalue_2)
          (`|ExecutionSequence`
            (:`then_0`
              (if (!= _index 0)
                ;;[1 1 1] Trace Upward
                (for _index_2 (range 5)
                  (bind _returnvalue_3 (+ (`self.K2_GetActorLocation`) (`KismetMathLibrary.MakeVector` (* _returnvalue_x (* _index_2 20)) (* (* _index_2 20) _returnvalue_y) 200.0)))
                  (bind (_outhit_2 _returnvalue_4) (`KismetSystemLibrary.SphereTraceSingle` :`Start` _returnvalue_3 :`End` (+ _returnvalue_3 (* (`self.GetActorUpVector`) -200.0)) :`Radius` 10.0 :`TraceChannel` "TraceTypeQuery1" :`DrawDebugType` "ForDuration"))
                  (if _returnvalue_4
                    (`|ExecutionSequence`
                      (:`then_0`
                        (bind (_bblockinghit _binitialoverlap _time _distance _location) (`GameplayStatics.BreakHitResult` _outhit_2))
                        ;;[1 1 1] Mantle Animation
                        (`KismetSystemLibrary.DrawDebugSphere` _location 10.0 12 (struct :`R` 1.0 :`B` 0.943703 :`A` 1.0) 10000.0 2.0)
                        (`MotionWarpingComponent.AddOrUpdateWarpTarget` (`self.MotionWarping`) (make `MotionWarpingTarget` "Mantle" (- _location (0.0 0.0 3.0)) (`self.K2_GetActorRotation`)))
                        (if (> (`KismetMathLibrary.Vector_Distance` _location (`SceneComponent.K2_GetComponentLocation` (`self.Mesh`))) 200.0)
                          (`|PlayMontage` _mesh "/Game/PoPCC/Characters/Prince/Animations/Mantle/Mantling_2M_Montage.Mantling_2M_Montage"
                            (:`then`
                              (`CharacterMovementComponent.SetMovementMode` _charactermovement "MOVE_Flying" 0 :!label _label_3)
                              (set `self.IsMantling` true)
                              ;;[1 1 1] Fix Capsule Height if crouching
                              (if (`self.IsCrouching`)
                                (`CapsuleComponent.SetCapsuleHalfHeight` (`self.CapsuleComponent`) 88.0 true)
                                (`SceneComponent.K2_SetRelativeLocation` (`self.Mesh`) (0.0 0.0 -89.0) false false)))
                            (:`OnCompleted`
                              (`CharacterMovementComponent.SetMovementMode` _charactermovement "MOVE_Walking" 0 :!label _label_4)
                              (set `self.IsMantling` false)
                              (if (`self.IsCrouching`)
                                (bind (_direction _capsule_height) (`Timeline|Timeline`)
                                  (:`Update`
                                    (`CapsuleComponent.SetCapsuleHalfHeight` (`self.CapsuleComponent`) (`KismetMathLibrary.Lerp` 88.0 50.0 _capsule_height) true)
                                    (`SceneComponent.K2_SetRelativeLocation` (`self.Mesh`) (`KismetMathLibrary.MakeVector` 0.0 0.0 (`KismetMathLibrary.Lerp` -89.0 -49.0)) false false))))))
                          (else
                            (`|PlayMontage` _mesh "/Game/PoPCC/Characters/Prince/Animations/Mantle/Mantling_1M_Montage.Mantling_1M_Montage"
                              (:`then`
                                (goto _label_3))
                              (:`OnCompleted`
                                (goto _label_4))))))
                      (:`then_1`
                        (break)))))))
            (:`then_1`
              (break))))))))

(fn `Uncrouch Obstacle`
  (returns (FoundObstacle :type Boolean))
  (bind _returnvalue (`self.K2_GetActorLocation`))
  (bind (_outhit _returnvalue_2) (`KismetSystemLibrary.SphereTraceSingle` :`Start` _returnvalue :`End` (+ _returnvalue (* (`KismetMathLibrary.GetUpVector` (`self.K2_GetActorRotation`)) 150.0)) :`Radius` 10.0 :`TraceChannel` "TraceTypeQuery1" :`DrawDebugType` "ForDuration"))
  (return _returnvalue_2))

(fn `UserConstructionScript`)