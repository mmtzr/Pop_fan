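; Player character Blueprint for the Prince, which spawns a follow camera and handles Enhanced Input movement, montage rolls and timeline-blended crouching with an overhead obstacle check.
; Jump runs a ledge trace and mantles or jumps, while the Mantle input sphere-traces for height-based climb montages.
; Both climbs use motion warping and Flying mode.
; Falls poll vertical speed to trigger hard landings; the falling ledge-trace timer is an empty stub.
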(event `self.ReceiveBeginPlay`
  (bind _returnvalue (`GameplayStatics.GetPlayerController` 0))
  ;[1 1 1] Main movement mapping input & camera spawn
  (`KismetSystemLibrary.PrintString` (`KismetStringLibrary.Conv_VectorToString` (`MovementComponent.Velocity` (`self.CharacterMovement`))))
  (bind _returnvalue_2 (`|SpawnActorFromClass` "/Game/PoPCC/Blueprints/BP_CameraManager.BP_CameraManager_C" (`KismetMathLibrary.MakeTransform` (`self.K2_GetActorLocation`)) "Undefined" "MultiplyWithRoot" null self null))
  (`PlayerController.SetViewTargetWithBlend` _returnvalue _returnvalue_2 0.0 "VTBlend_Linear" 0.0 false)
  (`EnhancedInputSubsystemInterface.AddMappingContext` (pcsubsystem `EnhancedInputLocalPlayerSubsystem` _returnvalue) "/Game/PoPCC/Input/IMC_PoPInput.IMC_PoPInput" 0 (struct)))

(event `Key|Q`
  (params (Key :type "Key Structure"))
  ;[1 1 1] Dirty Quit
  (:`Pressed`
    (`KismetSystemLibrary.QuitGame` null "Quit")))

(event `EnhancedInput|/Game/PoPCC/Input/IA_Movement`
  (params (ActionValue :type "Vector2D Structure") (ElapsedSeconds :type "Float (double-precision)") (TriggeredSeconds :type "Float (double-precision)") (InputAction :type "InputAction Object Reference" :default "/Game/PoPCC/Input/IA_Movement.IA_Movement"))
  ;[1 1 1] X&Y Movement
  (:`Triggered`
    (`self.AddMovementInput` (`KismetMathLibrary.GetRightVector` (`self.GetControlRotation`)) ActionValue_X)
    (`self.AddMovementInput` (`KismetMathLibrary.GetForwardVector` (`self.GetControlRotation`)) ActionValue_Y)))

(event `EnhancedInput|/Game/PoPCC/Input/IA_Roll`
  (params (ActionValue :type Boolean) (ElapsedSeconds :type "Float (double-precision)") (TriggeredSeconds :type "Float (double-precision)") (InputAction :type "InputAction Object Reference" :default "/Game/PoPCC/Input/IA_Roll.IA_Roll"))
  ;[1 1 1] Roll Dodge
  (:`Started`
    (if (not (`self.IsRolling`))
      (`|PlayMontage` (`self.Mesh`) "/Game/PoPCC/Characters/Prince/Animations/Roll/Roll_Montage.Roll_Montage"
        (:`then`
          (set `self.IsRolling` true))
        (:`OnCompleted`
          (set `self.IsRolling` false))))))

(event `EnhancedInput|/Game/PoPCC/Input/IA_Crouching`
  (params (ActionValue :type Boolean) (ElapsedSeconds :type "Float (double-precision)") (TriggeredSeconds :type "Float (double-precision)") (InputAction :type "InputAction Object Reference" :default "/Game/PoPCC/Input/IA_Crouching.IA_Crouching"))
  (bind _charactermovement (`self.CharacterMovement`))
  ;[1 1 1] Crouched Movement & Camera
  (:`Started`
    (if (not (`self.IsCrouching`))
      (set `self.IsCrouching` true)
      (set `CharacterMovementComponent.MaxWalkSpeed` 350.0 _charactermovement)
      (`|ExecutionSequence`
        (:`then_0`
          (bind (_direction _arm_length) (`Timeline|Crouched Zoom Out` :!label _label)
            (:`Update`
              (set `SpringArmComponent.TargetArmLength` (`KismetMathLibrary.Lerp` 600.0 750.0 _arm_length) (`self.CameraBoom`)))))
        (:`then_1`
          (bind (_direction_2 _capsule_height) (`Timeline|Crouched Capsule Height` :!label _label_2)
            (:`Update`
              (`CapsuleComponent.SetCapsuleHalfHeight` (`self.CapsuleComponent`) (`KismetMathLibrary.Lerp` 88.0 50.0 _capsule_height) true)
              (`SceneComponent.K2_SetRelativeLocation` (`self.Mesh`) (`KismetMathLibrary.MakeVector` 0.0 0.0 (`KismetMathLibrary.Lerp` -89.0 -49.0 _capsule_height)) false false)))))
      (else
        ;;[1 1 1] stop crouching if there is no obstacle
        (bind _foundobstacle (`self.Uncrouch Obstacle`))
        (if (not _foundobstacle)
          (set `self.IsCrouching` false)
          (set `CharacterMovementComponent.MaxWalkSpeed` 600.0 _charactermovement)
          (`|ExecutionSequence`
            (:`then_0`
              (goto _label :!via `Reverse`))
            (:`then_1`
              (goto _label_2 :!via `Reverse`))))))))

(event `EnhancedInput|/Game/ThirdPerson/Input/Actions/IA_Jump`
  (params (ActionValue :type Boolean) (ElapsedSeconds :type "Float (double-precision)") (TriggeredSeconds :type "Float (double-precision)") (InputAction :type "InputAction Object Reference" :default "/Game/ThirdPerson/Input/Actions/IA_Jump.IA_Jump"))
  ;[1 1 1] Jump & Mantle
  (:`Triggered`
    (if (not (`NavMovementComponent.IsFalling` (`self.CharacterMovement`)))
      (bind (_mantlepositiona _mantlepositionb) (`self.LedgeTrace` "ForDuration"))
      (if (`self.IsMantling`)
        (`self.Mantle` _mantlepositiona _mantlepositionb -100.0 30.0 1.0)
        (else
          (`self.Jump`))))))

(event `self.OnJumped`
  ;[1 1 1] Start tracing when player falls/jumps
  (bind _returnvalue (`KismetSystemLibrary.K2_SetTimer` null "TraceLedgeFalling" 0.1 true :!label _label_3))
  (set `self.FallingLedgeTraceHandle` _returnvalue))

(event `self.OnWalkingOffLedge`
  (params (PreviousFloorImpactNormal :type "Vector Structure (by ref)") (PreviousFloorContactNormal :type "Vector Structure (by ref)") (PreviousLocation :type "Vector Structure (by ref)") (TimeDelta :type "Float (single-precision)"))
  ;[1 1 1] Start tracing when player falls/jumps
  (goto _label_3))

(event `TraceLedgeFalling`
  (if (`self.FallingLedgeTrace`)
    _))

(event `EnhancedInput|/Game/PoPCC/Input/IA_Mantle`
  (params (ActionValue :type Boolean) (ElapsedSeconds :type "Float (double-precision)") (TriggeredSeconds :type "Float (double-precision)") (InputAction :type "InputAction Object Reference" :default "/Game/PoPCC/Input/IA_Mantle.IA_Mantle"))
  (bind (_returnvalue_x _returnvalue_y) (`KismetMathLibrary.BreakVector` (`self.GetActorForwardVector`)))
  (bind _charactermovement (`self.CharacterMovement`))
  (bind _mesh (`self.Mesh`))
  ;[1 1 1] Mantle
  (:`Started`
    (if (and (not (`NavMovementComponent.IsFalling` (`self.CharacterMovement`))) (not (`self.IsMantling`)))
      ;;[1 1 1] Trace Upward
      (for _index (range 5)
        (bind _returnvalue (+ (`self.K2_GetActorLocation`) (`KismetMathLibrary.MakeVector` (* _returnvalue_x (* _index 20)) (* (* _index 20) _returnvalue_y) 300.0)))
        (bind (_outhit _returnvalue_2) (`KismetSystemLibrary.SphereTraceSingle` :`Start` _returnvalue :`End` (+ _returnvalue (* (`self.GetActorUpVector`) -200.0)) :`Radius` 10.0 :`TraceChannel` "TraceTypeQuery1" :`DrawDebugType` "ForDuration"))
        (if _returnvalue_2
          (`|ExecutionSequence`
            (:`then_0`
              (bind (_bblockinghit _binitialoverlap _time _distance _location) (`GameplayStatics.BreakHitResult` _outhit))
              ;;[1 1 1] Mantle Animation
              (`KismetSystemLibrary.DrawDebugSphere` _location 10.0 12 (struct :`R` 1.0 :`B` 0.943703 :`A` 1.0) 10000.0 2.0)
              (`MotionWarpingComponent.AddOrUpdateWarpTarget` (`self.MotionWarping`) (make `MotionWarpingTarget` "Mantle" (- _location (0.0 0.0 3.0)) (`self.K2_GetActorRotation`)))
              (if (> (`KismetMathLibrary.Vector_Distance` _location (`SceneComponent.K2_GetComponentLocation` (`self.Mesh`))) 200.0)
                (`|PlayMontage` _mesh "/Game/PoPCC/Characters/Prince/Animations/Mantle/Mantling_2M_Montage.Mantling_2M_Montage"
                  (:`then`
                    (`CharacterMovementComponent.SetMovementMode` _charactermovement "MOVE_Flying" 0 :!label _label_4)
                    (set `self.IsMantling` true)
                    ;;[1 1 1] Fix Capsule Height if crouching
                    (if (`self.IsCrouching`)
                      (`CapsuleComponent.SetCapsuleHalfHeight` (`self.CapsuleComponent`) 88.0 true)
                      (`SceneComponent.K2_SetRelativeLocation` (`self.Mesh`) (0.0 0.0 -89.0) false false)))
                  (:`OnCompleted`
                    (`CharacterMovementComponent.SetMovementMode` _charactermovement "MOVE_Walking" 0 :!label _label_5)
                    (set `self.IsMantling` false)
                    (if (`self.IsCrouching`)
                      (bind (_direction _capsule_height) (`Timeline|Timeline`)
                        (:`Update`
                          (`CapsuleComponent.SetCapsuleHalfHeight` (`self.CapsuleComponent`) (`KismetMathLibrary.Lerp` 88.0 50.0 _capsule_height) true)
                          (`SceneComponent.K2_SetRelativeLocation` (`self.Mesh`) (`KismetMathLibrary.MakeVector` 0.0 0.0 (`KismetMathLibrary.Lerp` -89.0 -49.0)) false false))))))
                (else
                  (`|PlayMontage` _mesh "/Game/PoPCC/Characters/Prince/Animations/Mantle/Mantling_1M_Montage.Mantling_1M_Montage"
                    (:`then`
                      (goto _label_4))
                    (:`OnCompleted`
                      (goto _label_5))))))
            (:`then_1`
              (break))))))))

(event `SpeedCheck`
  (bind (_returnvalue_x _returnvalue_y _returnvalue_z) (`KismetMathLibrary.BreakVector` (`self.GetVelocity`)))
  ;[1 1 1] Hard Landing
  (if (<= _returnvalue_z -400.0) :!label _label_6
    (set `self.HardLanding` true)
    (else
      (`KismetSystemLibrary.Delay` 0.2)
      (`self.SpeedCheck`))))

(event `self.K2_OnMovementModeChanged`
  (params (PrevMovementMode :type "EMovementMode Enum" :default "MOVE_None") (NewMovementMode :type "EMovementMode Enum" :default "MOVE_None") (PrevCustomMode :type Byte) (NewCustomMode :type Byte))
  ;[1 1 1] Hard Landing
  (`|ExecutionSequence`
    (:`then_0`
      (if (`|EnumEquality` NewMovementMode "MOVE_Falling")
        (goto _label_6)))
    (:`then_1`
      (if (and (`|EnumEquality` NewMovementMode "MOVE_Walking") (`self.HardLanding`))
        (`CharacterMovementComponent.DisableMovement` (`self.CharacterMovement`))
        (bind _returnvalue (`self.PlayAnimMontage` "/Game/PoPCC/Characters/Prince/Animations/HardLand/HardLanding_UE_Montage.HardLanding_UE_Montage"))
        (set `self.HardLanding` false)
        (`KismetSystemLibrary.Delay` _returnvalue)
        (`CharacterMovementComponent.SetMovementMode` (`self.CharacterMovement`) "MOVE_Walking" 0)))))

(fn `LedgeTrace`
  (params (`Ledge Trace` :type "EDrawDebugTrace Enum" :default "None"))
  (returns (MantlePositionA :type "Vector Structure") (MantlePositionB :type "Vector Structure"))
  (locals (MantlePosA :type "Vector Structure") (MantlePosB :type "Vector Structure"))
  (bind _returnvalue (`self.K2_GetActorLocation`))
  (bind _returnvalue_2 (+ (`local.MantlePosB`) (0.0 0.0 100.0)))
  ;[1 1 1] Diagonal Trace for Ledge
  (bind (_outhit _returnvalue_3) (`KismetSystemLibrary.SphereTraceSingle` :`Start` _returnvalue :`End` (+ _returnvalue (* (`self.GetActorForwardVector`) 50.0) (0.0 0.0 250.0)) :`Radius` 10.0 :`TraceChannel` "TraceTypeQuery1" :`DrawDebugType` (`local.Ledge Trace`)))
  ;[1 1 1] Check if there is space above ledge to land
  (if _returnvalue_3
    (bind (_bblockinghit _binitialoverlap _time _distance _location _impactpoint) (`GameplayStatics.BreakHitResult` _outhit))
    (set `local.MantlePosA` (+ _impactpoint (* (`self.GetActorForwardVector`) -100.0)))
    (bind _output_get (set `local.MantlePosB` (+ _impactpoint (* (`self.GetActorForwardVector`) 10.0))))
    (set `self.IsMantling` true)
    (bind _returnvalue_4 (+ _output_get (0.0 0.0 20.0)))
    (bind (_outhit_2 _returnvalue_5) (`KismetSystemLibrary.SphereTraceSingle` _returnvalue_4 _returnvalue_4 10.0 "TraceTypeQuery1"))
    (if _returnvalue_5
      (set `self.IsMantling` false)
      (else
        (set `local.MantlePosB` (+ _impactpoint (* (`self.GetActorForwardVector`) 50.0)))))
    (if (or (== (`local.MantlePosA`) (0.0 0.0 0.0)) (== (`local.MantlePosB`) (0.0 0.0 0.0)))
      (set `self.IsMantling` false :!label _label)
      (else
        ;[1 1 1] Check if there is space between two points
        (bind (_outhit_3 _returnvalue_6) (`KismetSystemLibrary.SphereTraceSingle` :`Start` (- (`local.MantlePosA`) _returnvalue_2) :`End` _returnvalue_2 :`Radius` 10.0 :`TraceChannel` "TraceTypeQuery1" :`DrawDebugType` (`local.Ledge Trace`)))
        (if _returnvalue_6
          (goto _label)
          (else
            _))))
    (return (`local.MantlePosA`) (`local.MantlePosB`))))

(fn `MantleTrace`
  (params (InitialTraceLength :type "Float (double-precision)") (`SecondaryTraceZ Offset` :type "Float (double-precision)") (FallingHeightMultiplier :type "Float (double-precision)") (DebugTrace :type "EDrawDebugTrace Enum" :default "None"))
  (returns (MantlePositionA :type "Vector Structure") (MantlePositionB :type "Vector Structure"))
  (locals (MantlePosA :type "Vector Structure") (MantlePosB :type "Vector Structure"))
  (bind _returnvalue (`self.K2_GetActorLocation`))
  (bind (_mantleposa_x _mantleposa_y) (`KismetMathLibrary.BreakVector` (`local.MantlePosA`)))
  (bind _returnvalue_2 (+ (`local.MantlePosB`) (0.0 0.0 100.0)))
  (set `self.IsMantling` false)
  ;[1 1 1] Initial Climbable Surface Detection
  (bind (_outhit _returnvalue_3) (`KismetSystemLibrary.LineTraceSingle` :`Start` _returnvalue :`End` (+ _returnvalue (* (`self.GetActorForwardVector`) (`local.InitialTraceLength`))) :`TraceChannel` "TraceTypeQuery1" :`DrawDebugType` (`local.DebugTrace`)))
  ;[1 1 1] if object found then trace height; if player is falling then offset height
  (if _returnvalue_3
    (bind (_bblockinghit _binitialoverlap _time _distance _location) (`GameplayStatics.BreakHitResult` _outhit))
    (bind (_outhit_2 _returnvalue_4) (`KismetSystemLibrary.SphereTraceSingle` :`Start` (+ _location (`KismetMathLibrary.MakeVector` 0.0 0.0 (* (`local.SecondaryTraceZ Offset`) (`KismetMathLibrary.SelectFloat` (`local.FallingHeightMultiplier`) 1.0 (`NavMovementComponent.IsFalling` (`self.CharacterMovement`)))))) :`End` _location :`Radius` 10.0 :`TraceChannel` "TraceTypeQuery1" :`DrawDebugType` (`local.DebugTrace`)))
    ;[1 1 1] Set Mantle positions for motion wrapping
    (if _returnvalue_4
      (bind (_bblockinghit_2 _binitialoverlap_2 _time_2 _distance_2 _location_2 _impactpoint) (`GameplayStatics.BreakHitResult` _outhit_2))
      (set `local.MantlePosA` (+ _impactpoint (* (`self.GetActorForwardVector`) -50.0)))
      (bind _output_get (set `local.MantlePosB` (+ _impactpoint (* (`self.GetActorForwardVector`) 120.0))))
      ;[1 1 1] Check headspace to make sure the player can land
      (set `self.IsMantling` true)
      (bind _returnvalue_5 (+ _output_get (0.0 0.0 20.0)))
      (bind (_outhit_3 _returnvalue_6) (`KismetSystemLibrary.SphereTraceSingle` :`Start` _returnvalue_5 :`End` _returnvalue_5 :`Radius` 10.0 :`TraceChannel` "TraceTypeQuery1" :`DrawDebugType` (`local.DebugTrace`)))
      (if _returnvalue_6
        (set `self.IsMantling` false)
        (else
          (set `local.MantlePosB` (+ _impactpoint (* (`self.GetActorForwardVector`) 50.0)))))
      (if (or (== (`local.MantlePosA`) (0.0 0.0 0.0)) (== (`local.MantlePosB`) (0.0 0.0 0.0)))
        (set `self.IsMantling` false :!label _label)
        (else
          ;[1 1 1] Make sure there is empty space between two mantle positions in order to mantle
          (bind (_outhit_4 _returnvalue_7) (`KismetSystemLibrary.SphereTraceSingle` :`Start` (`KismetMathLibrary.MakeVector` _mantleposa_x _mantleposa_y (.z _returnvalue_2)) :`End` _returnvalue_2 :`Radius` 20.0 :`TraceChannel` "TraceTypeQuery1" :`DrawDebugType` (`local.DebugTrace`)))
          (if _returnvalue_7
            (goto _label)
            (else
              _))))
      (return (`local.MantlePosA`) (`local.MantlePosB`)))
    (else
      (set `self.IsMantling` false))))

(fn `Uncrouch Obstacle`
  (returns (FoundObstacle :type Boolean))
  (bind _returnvalue (`self.K2_GetActorLocation`))
  (bind (_outhit _returnvalue_2) (`KismetSystemLibrary.SphereTraceSingle` :`Start` _returnvalue :`End` (+ _returnvalue (* (`KismetMathLibrary.GetUpVector` (`self.K2_GetActorRotation`)) 150.0)) :`Radius` 10.0 :`TraceChannel` "TraceTypeQuery1" :`DrawDebugType` "ForDuration"))
  (return _returnvalue_2))

(fn `UserConstructionScript`)